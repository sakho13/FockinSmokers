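; Actor component that moves its owner along the level's stage spline at a set speed.
; On BeginPlay it takes the first BP_StageSpline actor found in the world.
; Each tick it adds speed times delta time to a travelled distance, then sets the owner's location to that world-space point on the spline without sweeping.
; A FollowRotation flag also applies the spline's rotation to the owner.
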(event EventBeginPlay
  (CallFunction|InitStageSpline))

(event EventTick
  (params (DeltaSeconds :type Float%20%28single-precision%29))
  (CallFunction|UpdateDistanceEverySec DeltaSeconds))

(fn InitStageSpline
  (bind _outactors (Actor|GetAllActorsOfClass "/Game/Blueprints/Stage/BP_StageSpline.BP_StageSpline_C"))
  (LocalVariables|Setsplines _outactors)
  (Variables|Default|SetStageSpline (Utilities|Array|Get(acopy) (LocalVariables|Getsplines))))

(fn UpdateDistanceEverySec
  (params (DeltaSeconds :type Float%20%28double-precision%29))
  (bind _output_get (Variables|Default|SetDistance (+ (* DeltaSeconds (Variables|Default|GetSpeed)) (Variables|Default|GetDistance))))
  (bind _output_get_2 (LocalVariables|Setspline (Actor|GetComponentbyClass (Variables|Default|GetStageSpline) "/Script/Engine.SplineComponent")))
  (LocalVariables|Setowner (Components|GetOwner))
  (LocalVariables|Setloc (Spline|GetLocationatDistanceAlongSpline _output_get_2 _output_get "World"))
  (LocalVariables|Setrot (Spline|GetRotationatDistanceAlongSpline _output_get_2 _output_get "World"))
  (Transformation|SetActorLocation (LocalVariables|Getowner) (LocalVariables|Getloc) false false)
  (if (Variables|Default|GetbFollowRotation)
    (Transformation|SetActorRotation (LocalVariables|Getowner) (LocalVariables|Getrot))))